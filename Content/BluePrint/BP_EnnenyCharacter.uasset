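; BP_EnnenyCharacter is an enemy character that takes damage from player projectiles and is destroyed when its life runs out.
; Capsule overlaps are cast to BP_FirstPersonProjectile, and only those flagged PlayerProjectile pass their Damage to LoseHp and are then destroyed.
; LoseHp subtracts from Life and destroys the enemy at zero or below.
; Overlaps with other actor types just print a cast failure message.
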(event `self.CapsuleComponent.OnComponentBeginOverlap`
  (params (OverlappedComponent :type "PrimitiveComponent Object Reference") (OtherActor :type "Actor Object Reference") (OtherComp :type "PrimitiveComponent Object Reference") (OtherBodyIndex :type Integer) (bFromSweep :type Boolean) (SweepResult :type "HitResult Structure (by ref)"))
  (bind _asbp_first_person_projectile (cast `/Game/FirstPerson/Blueprints/BP_FirstPersonProjectile` OtherActor)
    (:`then`
      (if (`/Game/FirstPerson/Blueprints/BP_FirstPersonProjectile.PlayerProjectile` _asbp_first_person_projectile)
        (`self.LoseHp` (`/Game/FirstPerson/Blueprints/BP_FirstPersonProjectile.Damage` _asbp_first_person_projectile))
        (`self.K2_DestroyActor` _asbp_first_person_projectile)))
    (:`CastFailed`
      (`KismetSystemLibrary.PrintString` "Cast Failed"))))

(fn `LoseHp`
  (params (Amount :type Integer))
  (bind _output_get (set `self.Life` (- (`self.Life`) Amount)))
  (if (<= _output_get 0)
    (`self.K2_DestroyActor`)))

(fn `UserConstructionScript`)